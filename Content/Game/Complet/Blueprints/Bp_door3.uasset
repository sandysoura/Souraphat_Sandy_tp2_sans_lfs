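; Door Blueprint that swings open and closed and shows a text prompt while the third-person character overlaps its collision.
; OpenDoor uses a FlipFlop to play or reverse a timeline that lerps the door's yaw from closed to a quarter turn.
; A separate OuvrirPorte event, gated by Ouvrable and Ouverte flags, clears Ouvrable and adds incremental yaw through a second timeline, so it runs only once unless re-enabled.
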(event `OuvrirPorte`
  (if (`self.ouvrable`)
    (if (not (`self.ouverte`))
      (set `self.ouvrable` false)
      (set `self.ouverte` false)
      (`Timeline|Chronologie_0`
        (:`Update`
          (`SceneComponent.K2_AddLocalRotation` (`self.door`) (struct :`Yaw` 1.0) false false))))))

(event `Open Door`
  (`/Engine/EditorBlueprintResources/StandardMacros.FlipFlop`
    (:`A`
      (bind (_direction _doorfloat) (`Timeline|Chronologie` :!via `PlayFromStart` :!label _label)
        (:`Update`
          (`SceneComponent.K2_SetRelativeRotation` (`self.door`) (`KismetMathLibrary.MakeRotator` 0.0 0.0 (`KismetMathLibrary.Lerp` 0.0 90.0 _doorfloat)) false false))))
    (:`B`
      (goto _label :!via `Reverse`))))

(event `self.collision.OnComponentBeginOverlap`
  (params (OverlappedComponent :type "PrimitiveComponent Object Reference") (OtherActor :type "Actor Object Reference") (OtherComp :type "PrimitiveComponent Object Reference") (OtherBodyIndex :type Integer) (bFromSweep :type Boolean) (SweepResult :type "HitResult Structure (by ref)"))
  (cast `/Game/ThirdPerson/Blueprints/BP_ThirdPersonCharacter` OtherActor)
  (`SceneComponent.SetHiddenInGame` (`self.text`) false false))

(event `self.collision.OnComponentEndOverlap`
  (params (OverlappedComponent :type "PrimitiveComponent Object Reference") (OtherActor :type "Actor Object Reference") (OtherComp :type "PrimitiveComponent Object Reference") (OtherBodyIndex :type Integer))
  (cast `/Game/ThirdPerson/Blueprints/BP_ThirdPersonCharacter` OtherActor)
  (`SceneComponent.SetHiddenInGame` (`self.text`) true false))

(fn `UserConstructionScript`)