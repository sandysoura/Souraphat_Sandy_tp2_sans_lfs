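; Key pickup actor (cle) that the player collects with the G key.
; Overlap with BP_ThirdPersonCharacter on its Collision component sets Iscollect, which lets G print a French pickup message and destroy the actor.
; HasKey is set on the character in the end-overlap event rather than on the key press, and that event also sets Iscollect true, so the flag is never cleared.
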(event `Key|G`
  (params (Key :type "Key Structure"))
  (:`Pressed`
    (if (`self.iscollect`)
      (`KismetSystemLibrary.PrintString` "Cle recupperer!")
      (`self.K2_DestroyActor`))))

(event `self.collision.OnComponentBeginOverlap`
  (params (OverlappedComponent :type "PrimitiveComponent Object Reference") (OtherActor :type "Actor Object Reference") (OtherComp :type "PrimitiveComponent Object Reference") (OtherBodyIndex :type Integer) (bFromSweep :type Boolean) (SweepResult :type "HitResult Structure (by ref)"))
  (cast `/Game/ThirdPerson/Blueprints/BP_ThirdPersonCharacter` OtherActor)
  (set `self.iscollect` true))

(event `self.collision.OnComponentEndOverlap`
  (params (OverlappedComponent :type "PrimitiveComponent Object Reference") (OtherActor :type "Actor Object Reference") (OtherComp :type "PrimitiveComponent Object Reference") (OtherBodyIndex :type Integer))
  (bind _asbp_third_person_character (cast `/Game/ThirdPerson/Blueprints/BP_ThirdPersonCharacter` OtherActor))
  (set `/Game/ThirdPerson/Blueprints/BP_ThirdPersonCharacter.HasKey` true _asbp_third_person_character)
  (set `self.iscollect` true))

(fn `UserConstructionScript`)