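; Door actor that swings open once and shows a text prompt when the third-person character is near.
; OuvrirPorte checks Ouvrable and Ouverte, then clears Ouvrable so it cannot run again; Ouverte is never set true.
; A timeline adds a fixed local rotation to the Door on each update, so the final angle depends on update count.
; Collision overlap begin and end events show and hide the Text component.
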(event `OuvrirPorte`
  ; Ourvir porte
  (if (`self.ouvrable`)
    (if (not (`self.ouverte`))
      (set `self.ouvrable` false)
      (set `self.ouverte` false)
      (`Timeline|Chronologie_0`
        (:`Update`
          (`SceneComponent.K2_AddLocalRotation` (`self.door`) (struct :`Yaw` 1.5) false false))))))

(event `self.Collision.OnComponentBeginOverlap`
  (params (OverlappedComponent :type "PrimitiveComponent Object Reference") (OtherActor :type "Actor Object Reference") (OtherComp :type "PrimitiveComponent Object Reference") (OtherBodyIndex :type Integer) (bFromSweep :type Boolean) (SweepResult :type "HitResult Structure (by ref)"))
  ; Texte porte
  (cast `/Game/ThirdPerson/Blueprints/BP_ThirdPersonCharacter` OtherActor)
  (`SceneComponent.SetHiddenInGame` (`self.text`) false false))

(event `self.Collision.OnComponentEndOverlap`
  (params (OverlappedComponent :type "PrimitiveComponent Object Reference") (OtherActor :type "Actor Object Reference") (OtherComp :type "PrimitiveComponent Object Reference") (OtherBodyIndex :type Integer))
  ; Texte porte
  (cast `/Game/ThirdPerson/Blueprints/BP_ThirdPersonCharacter` OtherActor)
  (`SceneComponent.SetHiddenInGame` (`self.text`) true false))

(fn `UserConstructionScript`)