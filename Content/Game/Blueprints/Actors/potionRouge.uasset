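; Red potion pickup actor that serves as a collectible artifact for the third-person character.
; Overlapping its Collision component sets the character's HasArtifact flag immediately and arms Iscollect, before any key press.
; Pressing Z while Iscollect is set prints a French "artifact retrieved" message and destroys the actor.
; End overlap also sets Iscollect to true, so Z collection stays available after the character walks away.
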(event `Key|Z`
  (params (Key :type "Key Structure"))
  (:`Pressed`
    (if (`self.iscollect`)
      (`KismetSystemLibrary.PrintString` "Artéfact récuperer!")
      (`self.K2_DestroyActor`))))

(event `self.collision.OnComponentBeginOverlap`
  (params (OverlappedComponent :type "PrimitiveComponent Object Reference") (OtherActor :type "Actor Object Reference") (OtherComp :type "PrimitiveComponent Object Reference") (OtherBodyIndex :type Integer) (bFromSweep :type Boolean) (SweepResult :type "HitResult Structure (by ref)"))
  (bind _asbp_third_person_character (cast `/Game/ThirdPerson/Blueprints/BP_ThirdPersonCharacter` OtherActor))
  (set `/Game/ThirdPerson/Blueprints/BP_ThirdPersonCharacter.HasArtifact` true _asbp_third_person_character)
  (set `self.iscollect` true))

(event `self.collision.OnComponentEndOverlap`
  (params (OverlappedComponent :type "PrimitiveComponent Object Reference") (OtherActor :type "Actor Object Reference") (OtherComp :type "PrimitiveComponent Object Reference") (OtherBodyIndex :type Integer))
  (cast `/Game/ThirdPerson/Blueprints/BP_ThirdPersonCharacter` OtherActor)
  (set `self.iscollect` true))

(fn `UserConstructionScript`)