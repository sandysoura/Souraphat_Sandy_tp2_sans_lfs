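; Bookkey is a collectible artifact actor that the player picks up by pressing X while inside its Collision volume.
; Overlap by BP_ThirdPersonCharacter immediately sets that character's HasArtifact2 flag, before any key press, and raises a local Artefact flag that clears on exit.
; With input enabled for player controller 0, X checks that flag, prints a French pickup message and destroys the actor.
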(event `self.ReceiveBeginPlay`
  (`self.EnableInput` (`GameplayStatics.GetPlayerController` 0)))

(event `Key|X`
  (params (Key :type "Key Structure"))
  (:`Pressed`
    (if (`self.artefact`)
      (`KismetSystemLibrary.PrintString` "Artéfact recuperer!")
      (`self.K2_DestroyActor`))))

(event `self.Collision.OnComponentBeginOverlap`
  (params (OverlappedComponent :type "PrimitiveComponent Object Reference") (OtherActor :type "Actor Object Reference") (OtherComp :type "PrimitiveComponent Object Reference") (OtherBodyIndex :type Integer) (bFromSweep :type Boolean) (SweepResult :type "HitResult Structure (by ref)"))
  (bind _asbp_third_person_character (cast `/Game/ThirdPerson/Blueprints/BP_ThirdPersonCharacter` OtherActor))
  (set `/Game/ThirdPerson/Blueprints/BP_ThirdPersonCharacter.HasArtifact2` true _asbp_third_person_character)
  (set `self.artefact` true))

(event `self.Collision.OnComponentEndOverlap`
  (params (OverlappedComponent :type "PrimitiveComponent Object Reference") (OtherActor :type "Actor Object Reference") (OtherComp :type "PrimitiveComponent Object Reference") (OtherBodyIndex :type Integer))
  (cast `/Game/ThirdPerson/Blueprints/BP_ThirdPersonCharacter` OtherActor)
  (set `self.artefact` false))

(fn `UserConstructionScript`)