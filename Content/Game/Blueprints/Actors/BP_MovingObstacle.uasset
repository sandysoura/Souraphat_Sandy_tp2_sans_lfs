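; BP_MovingObstacle is a moving obstacle that kills the third-person character on contact.
; At BeginPlay it adds DestinationLocation as a relative control point to its InterpToMovement component, which drives the translation.
; A Box overlap calls Mort on the character, then a DoOnce spawns a particle emitter at its location and opens ThirdPersonMap after a short delay.
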(event `self.ReceiveBeginPlay`
  ; Mouvement translation des obstacles
  (`InterpToMovementComponent.AddControlPointPosition` (`self.InterpToMovement`) (`self.Destination Location`) true))

(event `self.Box.OnComponentBeginOverlap`
  (params (OverlappedComponent :type "PrimitiveComponent Object Reference") (OtherActor :type "Actor Object Reference") (OtherComp :type "PrimitiveComponent Object Reference") (OtherBodyIndex :type Integer) (bFromSweep :type Boolean) (SweepResult :type "HitResult Structure (by ref)"))
  ; Mouvement translation des obstacles
  (bind _asbp_third_person_character (cast `/Game/ThirdPerson/Blueprints/BP_ThirdPersonCharacter` OtherActor))
  (`/Game/ThirdPerson/Blueprints/BP_ThirdPersonCharacter.mort` _asbp_third_person_character)
  (`/Engine/EditorBlueprintResources/StandardMacros.DoOnce` false
    (:`Completed`
      (`GameplayStatics.SpawnEmitterAtLocation` null (`self.K2_GetActorLocation` _asbp_third_person_character))
      (`KismetSystemLibrary.Delay` 3.0)
      (`GameplayStatics.OpenLevel` "ThirdPersonMap"))))

(fn `UserConstructionScript`)